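; BPC_Health is a health component that tracks the current health of the actor it is attached to.
; RemoveHealth subtracts a damage amount and AddHealth adds a heal amount, each clamping CurrentHealth between MinHealth and MaxHealth.
; The event graph holds only disabled placeholder events, and neither function broadcasts changes or handles death.
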(fn `AddHealth`
  (params (HealAmount :type "Float (double-precision)"))
  (set `self.CurrentHealth` (`KismetMathLibrary.FClamp` (+ HealAmount (`self.CurrentHealth`)) (`self.MinHealth`) (`self.MaxHealth`))))

(fn `RemoveHealth`
  (params (DamageAmount :type "Float (double-precision)"))
  (set `self.CurrentHealth` (`KismetMathLibrary.FClamp` (- (`self.CurrentHealth`) DamageAmount) (`self.MinHealth`) (`self.MaxHealth`))))