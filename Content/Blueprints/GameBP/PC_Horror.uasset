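; PC_Horror is the player controller for a horror game, handling camera look and the inventory menu.
; On BeginPlay it creates a collapsed W_InventoryMenu widget, and look axes feed pitch and yaw scaled by LookSensitivity.
; The AccessInventory action toggles the menu through an IsPaused flag, switching character movement, look input, mouse cursor and input mode rather than pausing the game itself.
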(event `self.ReceiveBeginPlay`
  (bind _returnvalue (`|CreateWidget` "/Game/UMG/Inventory/W_InventoryMenu.W_InventoryMenu_C"))
  (bind _output_get (set `self.InventoryMenuReference` _returnvalue))
  (`Widget.SetVisibility` _output_get "Collapsed")
  (`UserWidget.AddToViewport` (`self.InventoryMenuReference`) 0))

(event `InputAxis|LookUp`
  (params (AxisValue :type "Float (single-precision)"))
  (`self.AddPitchInput` (* AxisValue (`self.LookSensitivity`))))

(event `InputAxis|LookRight`
  (params (AxisValue :type "Float (single-precision)"))
  (`self.AddYawInput` (* AxisValue (`self.LookSensitivity`))))

(event `InputAction|AccessInventory`
  (params (Key :type "Key Structure"))
  (:`Pressed`
    (`self.ToggleInventory`)))

(event `ToggleInventory`
  (bind _inventorymenureference (`self.InventoryMenuReference`))
  (bind _charactermovement (`Character.CharacterMovement` (`GameplayStatics.GetPlayerCharacter` 0)))
  (if (`self.IsPaused`)
    (set `self.IsPaused` false)
    (`CharacterMovementComponent.SetMovementMode` _charactermovement "MOVE_Walking" 0)
    (`self.ResetIgnoreLookInput`)
    (set `self.bShowMouseCursor` false)
    (`Widget.SetVisibility` _inventorymenureference "Collapsed")
    (`WidgetBlueprintLibrary.SetInputMode_GameOnly` self)
    (else
      (set `self.IsPaused` true)
      (`CharacterMovementComponent.DisableMovement` _charactermovement)
      (`self.SetIgnoreLookInput` true)
      (set `self.bShowMouseCursor` true)
      (`Widget.SetVisibility` _inventorymenureference "SelfHitTestInvisible")
      (`WidgetBlueprintLibrary.SetInputMode_GameAndUIEx` self _inventorymenureference))))

(fn `UserConstructionScript`)