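; Interactable door actor that swings open away from the player when used and closes on the next interaction.
; Interact alternates through a FlipFlop between playing and reversing the DoorOpenTime timeline.
; On opening, a dot product of the player-to-door direction and the actor's forward vector picks the swing side.
; The timeline lerps the Door's relative yaw from closed to a quarter turn in that direction.
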(event `/Game/Blueprints/Interfaces/BPI_Interaction.Interact`
  (`/Engine/EditorBlueprintResources/StandardMacros.FlipFlop`
    (:`A`
      (set `self.DotProduct` (`KismetMathLibrary.Dot_VectorVector` (`KismetMathLibrary.Normal` (- (`self.K2_GetActorLocation`) (`self.K2_GetActorLocation` (`self.PlayerReference`)))) (`self.GetActorForwardVector`)))
      (bind (_direction _newtrack_0) (`Timeline|DoorOpenTime` :!label _label)
        (:`Update`
          (`SceneComponent.K2_SetRelativeRotation` (`self.Door`) (`KismetMathLibrary.MakeRotator` 0.0 0.0 (`KismetMathLibrary.Lerp` 0.0 (select `bool` (>= (`self.DotProduct`) 0.0) :`false` -90.0 :`true` 90.0 :!type "Float (single-precision)") _newtrack_0)) false false))))
    (:`B`
      (goto _label :!via `Reverse`))))

(fn `UserConstructionScript`
  (`parent.UserConstructionScript`))