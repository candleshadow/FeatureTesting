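; Bandages inventory item that heals the player when used.
; UseItem adds HealAmount through the player's BPCHealth component when current health differs from max, and sets SuccessUse to report whether the heal was applied.
; It also prints the current health as debug output on each use.
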(event `self.UseItem`
  (bind _bpc_health (`/Game/Blueprints/GameBP/Level1/L1_Character.BPC_Health` (`self.PlayerReference`)))
  (bind _currenthealth (`/Game/Blueprints/BlueprintComponents/BPC_Health.CurrentHealth` _bpc_health))
  (if (!= _currenthealth (`/Game/Blueprints/BlueprintComponents/BPC_Health.MaxHealth` _bpc_health))
    (`/Game/Blueprints/BlueprintComponents/BPC_Health.AddHealth` _bpc_health (`self.Heal Amount`))
    (set `self.SuccessUse` true)
    (else
      (set `self.SuccessUse` false)))
  (`KismetSystemLibrary.PrintString` (`KismetStringLibrary.Conv_DoubleToString` _currenthealth)))

(fn `UserConstructionScript`
  (`parent.UserConstructionScript`))