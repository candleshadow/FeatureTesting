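; Actor component that gives the player a battery-powered flashlight, working on a light taken from the player reference passed at initialization.
; Toggling on requires charge above minimum and starts a looping timer that drains the battery, switching the light off when empty.
; IES brightness scale follows charge, fading only below one fifth of maximum.
; Battery replacement ignores its Amount input and updates brightness before refilling to maximum.
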(fn `DepleteBatteryLife`
  (bind _output_get (set `self.CurrentBatteryLevel` (`KismetMathLibrary.FClamp` (- (`self.CurrentBatteryLevel`) (`self.DepletionRate`)) (`self.MinBatteryLevel`) (`self.MaxBatteryLevel`))))
  (`self.SetIntensity`)
  (if (<= _output_get (`self.MinBatteryLevel`))
    (`self.ToggleFlashlight`)))

(fn `InitializeFlashlight`
  (params (Player :type "/Game/Blueprints/GameBP/Level1/L1_Character Object Reference"))
  (bind _output_get (set `self.PlayerReference` Player))
  (set `self.Flashlight` (`/Game/Blueprints/GameBP/Level1/L1_Character.Flashlight` _output_get)))

(fn `ReplaceBattery`
  (params (Amount :type "Float (double-precision)"))
  ;[0.9561 0.4672 1] Replacing a battery puts the current back to max
  (`self.SetIntensity`)
  (set `self.CurrentBatteryLevel` (`self.MaxBatteryLevel`)))

(fn `SetIntensity`
  (`LightComponent.SetIESBrightnessScale` (`self.Flashlight`) (`KismetMathLibrary.MapRangeClamped` (`self.CurrentBatteryLevel`) (`self.MinBatteryLevel`) (/ (`self.MaxBatteryLevel`) 5.0) 0.0 1.0)))

(fn `ToggleFlashlight`
  (bind _flashlight (`self.Flashlight`))
  (if (`SceneComponent.bVisible` _flashlight)
    (`SceneComponent.SetVisibility` _flashlight false false)
    (`KismetSystemLibrary.K2_ClearTimer` null "DepleteBatteryLife")
    (elif (> (`self.CurrentBatteryLevel`) (`self.MinBatteryLevel`))
      (`SceneComponent.SetVisibility` _flashlight true false)
      (`KismetSystemLibrary.K2_SetTimer` null "DepleteBatteryLife" (`self.DepletionTimer`) true))))