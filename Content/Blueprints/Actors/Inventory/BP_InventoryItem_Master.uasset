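; BP_InventoryItem_Master is the base actor for items the player picks up into their inventory.
; On Interact, it casts the instigator to L1_Character and passes its Item and Amount to that character's BPCInventory component.
; A successful add either leaves the remainder in the actor as the new Amount or destroys the actor.
; It caches a player reference on BeginPlay, and its UseItem event is empty.
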(event `self.ReceiveBeginPlay`
  (set `self.PlayerReference` (cast `/Game/Blueprints/GameBP/Level1/L1_Character` (`GameplayStatics.GetPlayerCharacter` 0) :!pure true)))

(event `/Game/Blueprints/Interfaces/BPI_Interaction.Interact`
  (params (Instigator :type "Pawn Object Reference"))
  (bind _asl1_character (cast `/Game/Blueprints/GameBP/Level1/L1_Character` Instigator))
  (bind (_success _remainder) (`/Game/Blueprints/BlueprintComponents/BPC_Inventory.AddItem` (`/Game/Blueprints/GameBP/Level1/L1_Character.BPC_Inventory` _asl1_character) (`self.Item`) (`self.Amount`)))
  (if _success
    (if (> _remainder 0)
      (set `self.Amount` _remainder)
      (else
        (`self.K2_DestroyActor`)))))

(event `UseItem`)

(fn `UserConstructionScript`)